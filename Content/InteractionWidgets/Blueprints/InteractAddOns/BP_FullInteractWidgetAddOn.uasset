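; Interaction add-on actor that shows a world-space BP_MasterInteractionWidget for its parent actor, which it assigns as the widget's interaction actor.
; When given a target pawn while toggled on, it turns the offset toward the pawn, fits draw size to the widget and shrinks render scale with distance.
; Toggling or clearing the target hides the widget.
; The widget content functions (title, type, details and the like) return only default values here.
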(event `/Game/InteractionWidgets/Blueprints/Interfaces/InteractionInterface.Clear Target`
  ;[1 1 1] Clear target
  (`SceneComponent.SetVisibility` (`self.Widget`) false false))

(event `/Game/InteractionWidgets/Blueprints/Interfaces/InteractionInterface.Toggle Widget`
  (params (Widget :type Boolean))
  ;[1 1 1] Toggle widget
  (`self.Server Toggle Widget` Widget))

(event `self.ReceiveBeginPlay`
  ;[1 1 1] Set widgets interaction actor
  (set `/Game/InteractionWidgets/Blueprints/Widgets/BP_MasterInteractionWidget.Interaction Actor` (`self.GetParentActor`) (cast `/Game/InteractionWidgets/Blueprints/Widgets/BP_MasterInteractionWidget` (`WidgetComponent.GetUserWidgetObject` (`self.Widget`)) :!pure true)))

(event `Server Toggle Widget`
  (params (`Widget Toggle` :type Boolean))
  ;[1 1 1] Server toggle widget
  (set `self.Widget Toggle` `Widget Toggle`)
  (`/Game/InteractionWidgets/Blueprints/Interfaces/InteractionInterface.Clear Target`))

(event `/Game/InteractionWidgets/Blueprints/Interfaces/InteractionInterface.ParentActor`
  (params (Actor :type "Actor Object Reference"))
  (set `/Game/InteractionWidgets/Blueprints/Widgets/BP_MasterInteractionWidget.Interaction Actor` Actor (cast `/Game/InteractionWidgets/Blueprints/Widgets/BP_MasterInteractionWidget` (`WidgetComponent.GetUserWidgetObject` (`self.Widget`)) :!pure true)))

(event `/Game/InteractionWidgets/Blueprints/Interfaces/InteractionInterface.Current Target`
  (params (Pawn :type "Pawn Object Reference"))
  (bind (_returnvalue_x _returnvalue_y) (`KismetMathLibrary.BreakVector` (`SceneComponent.K2_GetComponentScale` (`self.Widget`))))
  (bind (_x _y) (`KismetMathLibrary.BreakVector2D` (`Widget.GetDesiredSize` (cast `/Game/InteractionWidgets/Blueprints/Widgets/BP_MasterInteractionWidget` (`WidgetComponent.GetUserWidgetObject` (`self.Widget`)) :!pure true))))
  (bind _returnvalue (`KismetMathLibrary.MapRangeClamped` (`KismetMathLibrary.VSize` (- (`self.K2_GetActorLocation`) (`self.K2_GetActorLocation` (`self.Target Pawn`)))) 400.0 650.0 1.0 0.6))
  ;[1 1 1] Current target
  (set `self.Target Pawn` Pawn)
  (bind _asbp_master_interaction_widget (cast `/Game/InteractionWidgets/Blueprints/Widgets/BP_MasterInteractionWidget` (`WidgetComponent.GetUserWidgetObject` (`self.Widget`))))
  (set `/Game/InteractionWidgets/Blueprints/Widgets/BP_MasterInteractionWidget.Interaction Actor` (`self.GetParentActor`) _asbp_master_interaction_widget)
  ;[1 1 1] Is widget toggled on
  (if (`self.Widget Toggle`)
    ;[1 1 1] Set the widget offset rotation
    (`SceneComponent.K2_SetWorldRotation` (`self.Widget Offset`) (`KismetMathLibrary.FindLookAtRotation` (`SceneComponent.K2_GetComponentLocation` (`self.Widget Offset`)) (`self.K2_GetActorLocation` (`self.Target Pawn`))) false false)
    ;[1 1 1] Set widget visibility
    (`SceneComponent.SetVisibility` (`self.Widget`) true false)
    ;[1 1 1] Set the draw size of the widget
    (`WidgetComponent.SetDrawSize` (`self.Widget`) (`KismetMathLibrary.MakeVector2D` _x _y))
    ;[1 1 1] Set the widget world scale, reduce from far distances
    (`Widget.SetRenderScale` (`WidgetComponent.GetUserWidgetObject` (`self.Widget`)) (`KismetMathLibrary.MakeVector2D` (* _returnvalue_x _returnvalue) (* _returnvalue_y _returnvalue)))
    (else
      (`SceneComponent.SetVisibility` (`self.Widget`) false false))))

(fn `Set Detail 1`
  (returns (`Return Value` :type Boolean) (`Detail Settings` :type "/Game/InteractionWidgets/Blueprints/Stucts/S_DetailsSettings Structure"))
  (return false))

(fn `Set Detail 2`
  (returns (`Return Value` :type Boolean) (`Detail Settings` :type "/Game/InteractionWidgets/Blueprints/Stucts/S_DetailsSettings Structure"))
  (return false))

(fn `Set Detail 3`
  (returns (`Return Value` :type Boolean) (`Detail Settings` :type "/Game/InteractionWidgets/Blueprints/Stucts/S_DetailsSettings Structure"))
  (return false))

(fn `Set Detail 4`
  (returns (`Return Value` :type Boolean) (`Detail Settings` :type "/Game/InteractionWidgets/Blueprints/Stucts/S_DetailsSettings Structure"))
  (return false))

(fn `Set Widget Amount`
  (returns (`Return Value` :type Boolean) (`Amount Value` :type Integer))
  (return false 0))

(fn `Set Widget Color`
  (returns (`Dark Color` :type "LinearColor Structure") (`Light Color` :type "LinearColor Structure"))
  (return))

(fn `Set Widget Key Binds`
  (returns (`Return Value` :type Boolean) (`Key Binds` :type "Array of /Game/InteractionWidgets/Blueprints/Stucts/S_KeyBinds Structure"))
  (return false))

(fn `Set Widget Level`
  (returns (`Return Value` :type Boolean) (`Level Text` :type Text))
  (return false ""))

(fn `Set Widget Sub Title`
  (returns (`Return Value` :type Boolean) (`Sub Title Text` :type Text))
  (return false ""))

(fn `Set Widget Title`
  (returns (`Return Value` :type Boolean) (`Title Text` :type Text))
  (return false ""))

(fn `Set Widget Type`
  (returns (`Widget Type` :type "/Game/InteractionWidgets/Blueprints/Enums/E_WidgetTypes Enum"))
  (return "NewEnumerator0"))

(fn `UserConstructionScript`
  ;[1 1 1] Set widget offset size
  (`SceneComponent.K2_SetRelativeLocation` (`self.Widget`) (`KismetMathLibrary.MakeVector` 0.0 (`self.Widget Offset Size`)) false false))