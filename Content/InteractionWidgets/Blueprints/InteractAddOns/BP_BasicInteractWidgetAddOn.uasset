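; BP_BasicInteractWidgetAddOn is an add-on actor that displays an interaction widget for its parent actor.
; On BeginPlay it passes the parent actor to the master interaction widget.
; When targeted and toggled on, it rotates the offset pivot to face the pawn, resizes the widget to its content and scales it down with distance.
; Clearing the target hides it, and the widget detail getters return only empty defaults.
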(event `self.ReceiveBeginPlay`
  ;[1 1 1] Set widgets interaction actor
  (set `/Game/InteractionWidgets/Blueprints/Widgets/BP_MasterInteractionWidget.Interaction Actor` (`self.GetParentActor`) (cast `/Game/InteractionWidgets/Blueprints/Widgets/BP_MasterInteractionWidget` (`WidgetComponent.GetUserWidgetObject` (`self.Widget`)) :!pure true))
  ;[1 1 1] Set widget offset
  (`SphereComponent.SetSphereRadius` (`self.Widget Offset`) (`self.Widget Offset Size`) false))

(event `/Game/InteractionWidgets/Blueprints/Interfaces/InteractionInterface.Toggle Widget`
  (params (Widget :type Boolean))
  ;[1 1 1] Toggle the widget
  (set `self.Widget Toggle` Widget))

(event `/Game/InteractionWidgets/Blueprints/Interfaces/InteractionInterface.Clear Target`
  ;[1 1 1] Clear target
  ;[1 1 1] Hide widget
  (`SceneComponent.SetVisibility` (`self.Widget`) false false))

(event `/Game/InteractionWidgets/Blueprints/Interfaces/InteractionInterface.Current Target`
  (params (Pawn :type "Pawn Object Reference"))
  (bind (_returnvalue_x _returnvalue_y) (`KismetMathLibrary.BreakVector` (`SceneComponent.K2_GetComponentScale` (`self.Widget`))))
  (bind (_x _y) (`KismetMathLibrary.BreakVector2D` (`Widget.GetDesiredSize` (cast `/Game/InteractionWidgets/Blueprints/Widgets/BP_MasterInteractionWidget` (`WidgetComponent.GetUserWidgetObject` (`self.Widget`)) :!pure true))))
  (bind _returnvalue (`KismetMathLibrary.MapRangeClamped` (`KismetMathLibrary.VSize` (- (`self.K2_GetActorLocation`) (`self.K2_GetActorLocation` (`self.Target Pawn`)))) 400.0 650.0 1.0 0.6))
  ;[1 1 1] Current target
  (set `self.Target Pawn` Pawn)
  ;[1 1 1] Current target events
  (if (`self.Widget Toggle`)
    (`SceneComponent.K2_SetWorldRotation` (`self.Widget Offset`) (`KismetMathLibrary.FindLookAtRotation` (`SceneComponent.K2_GetComponentLocation` (`self.Widget Offset`)) (`self.K2_GetActorLocation` (`self.Target Pawn`))) false false)
    (`SceneComponent.SetVisibility` (`self.Widget`) true false)
    (`WidgetComponent.SetDrawSize` (`self.Widget`) (`KismetMathLibrary.MakeVector2D` _x _y))
    (`Widget.SetRenderScale` (`WidgetComponent.GetUserWidgetObject` (`self.Widget`)) (`KismetMathLibrary.MakeVector2D` (* _returnvalue_x _returnvalue) (* _returnvalue_y _returnvalue)))
    (else
      (`SceneComponent.SetVisibility` (`self.Widget`) false false))))

(fn `Set Detail 1`
  (returns (`Return Value` :type Boolean) (`Detail Settings` :type "/Game/InteractionWidgets/Blueprints/Stucts/S_DetailsSettings Structure"))
  (return false))

(fn `Set Detail 2`
  (returns (`Return Value` :type Boolean) (`Detail Settings` :type "/Game/InteractionWidgets/Blueprints/Stucts/S_DetailsSettings Structure"))
  (return false))

(fn `Set Detail 3`
  (returns (`Return Value` :type Boolean) (`Detail Settings` :type "/Game/InteractionWidgets/Blueprints/Stucts/S_DetailsSettings Structure"))
  (return false))

(fn `Set Detail 4`
  (returns (`Return Value` :type Boolean) (`Detail Settings` :type "/Game/InteractionWidgets/Blueprints/Stucts/S_DetailsSettings Structure"))
  (return false))

(fn `Set Widget Amount`
  (returns (`Return Value` :type Boolean) (`Amount Value` :type Integer))
  (return false 0))

(fn `Set Widget Color`
  (returns (`Dark Color` :type "LinearColor Structure") (`Light Color` :type "LinearColor Structure"))
  (return))

(fn `Set Widget Key Binds`
  (returns (`Return Value` :type Boolean) (`Key Binds` :type "Array of /Game/InteractionWidgets/Blueprints/Stucts/S_KeyBinds Structure"))
  (return false))

(fn `Set Widget Level`
  (returns (`Return Value` :type Boolean) (`Level Text` :type Text))
  (return false ""))

(fn `Set Widget Sub Title`
  (returns (`Return Value` :type Boolean) (`Sub Title Text` :type Text))
  (return false ""))

(fn `Set Widget Title`
  (returns (`Return Value` :type Boolean) (`Title Text` :type Text))
  (return false ""))

(fn `Set Widget Type`
  (returns (`Widget Type` :type "/Game/InteractionWidgets/Blueprints/Enums/E_WidgetTypes Enum"))
  (return "NewEnumerator0"))

(fn `UserConstructionScript`
  ;[1 1 1] Set widget offset size
  (`SceneComponent.K2_SetRelativeLocation` (`self.Widget`) (`KismetMathLibrary.MakeVector` 0.0 (`self.Widget Offset Size`)) false false))