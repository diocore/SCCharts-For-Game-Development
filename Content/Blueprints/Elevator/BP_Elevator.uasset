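; BP_Elevator is the main actor of a three-floor elevator demonstration that interfaces with SCCharts state-machine logic.
; Construction wires the child-actor room, outside doors and call buttons back to it.
; Its events relay door and movement commands, update button status, and report room door status to the SCCharts wrapper after a fixed animation delay.
; A debug Tick swaps state-chart images on a screen widget as DebugStateID changes.
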(event `self.OpenOutsideDoors`
  (params (floor :type Integer))
  (bind _doorsatfloor0 (`self.DoorsAtFloor0`))
  (bind _doorsatfloor1 (`self.DoorsAtFloor1`))
  (bind _doorsatfloor2 (`self.DoorsAtFloor2`))
  ;[1 1 1] This opens the outside doors of the floors at the given floor and plaus an audio when ever it opens a floor.
  (`|ExecutionSequence`
    (:`then_0`
      (switch `int` floor
        (:`0`
          (`/Game/Blueprints/Elevator/DoorsOuter/BP_ElevatorDoorOutside.OpenDoors` _doorsatfloor0)
          (`AddComponent|NODE_AddAudioComponent-4` :`RelativeTransform` (`self.GetTransform` _doorsatfloor0))
          (bind _asbp_btn_base (cast `/Game/Blueprints/Elevator/BbtnPanel/BP_BtnBase` (`ChildActorComponent.ChildActor` (`self.BP_BtnUpOutside`))))
          (`/Game/Blueprints/Elevator/BbtnPanel/BP_BtnBase.SetStatus` _asbp_btn_base false))
        (:`1`
          (`/Game/Blueprints/Elevator/DoorsOuter/BP_ElevatorDoorOutside.OpenDoors` _doorsatfloor1)
          (`AddComponent|NODE_AddAudioComponent-5` :`RelativeTransform` (`self.GetTransform` _doorsatfloor1))
          (bind _asbp_btn_base_2 (cast `/Game/Blueprints/Elevator/BbtnPanel/BP_BtnBase` (`ChildActorComponent.ChildActor` (`self.BP_BtnUpOutside1`))))
          (`/Game/Blueprints/Elevator/BbtnPanel/BP_BtnBase.SetStatus` _asbp_btn_base_2 false))
        (:`2`
          (`/Game/Blueprints/Elevator/DoorsOuter/BP_ElevatorDoorOutside.OpenDoors` _doorsatfloor2)
          (`AddComponent|NODE_AddAudioComponent-6` :`RelativeTransform` (`self.GetTransform` _doorsatfloor2))
          (bind _asbp_btn_base_3 (cast `/Game/Blueprints/Elevator/BbtnPanel/BP_BtnBase` (`ChildActorComponent.ChildActor` (`self.BP_BtnUpOutside2`))))
          (`/Game/Blueprints/Elevator/BbtnPanel/BP_BtnBase.SetStatus` _asbp_btn_base_3 false))))
    (:`then_1`
      (`/Game/Blueprints/Elevator/elevatorRoom/BP_ElevatorRoom.SetStatus` (`self.BP Elevator Room`) floor false))))

(event `self.CloseOutsideDoors`
  (params (floor :type Integer))
  ;[1 1 1] This closes the outside doors at the given floor
  (switch `int` floor
    (:`0`
      (`/Game/Blueprints/Elevator/DoorsOuter/BP_ElevatorDoorOutside.CloseDoors` (`self.DoorsAtFloor0`)))
    (:`1`
      (`/Game/Blueprints/Elevator/DoorsOuter/BP_ElevatorDoorOutside.CloseDoors` (`self.DoorsAtFloor1`)))
    (:`2`
      (`/Game/Blueprints/Elevator/DoorsOuter/BP_ElevatorDoorOutside.CloseDoors` (`self.DoorsAtFloor2`)))))

(event `self.MoveElevator`
  (params (up :type Boolean) (numOfFloors :type Integer))
  ;[1 1 1] Move Elevator relays the move comment from the main Elevator Actor to the Elevator room, which is then moves itself by the number of floors given in the direction up or down
  (bind _asbp_elevator_room (cast `/Game/Blueprints/Elevator/elevatorRoom/BP_ElevatorRoom` (`ChildActorComponent.ChildActor` (`self.BP_ElevatorRoom`))))
  (`/Game/Blueprints/Elevator/elevatorRoom/BP_ElevatorRoom.MoveElevator` _asbp_elevator_room up numOfFloors))

(event `self.OpenElevatorRoomDoors`
  ;[1 1 1] This handels the opening/closing of the Elevator Rooms doors. There is A Delay to wait for before the updated status is send to the SCCharts wrapper function UpdateDoorStatus to make sure the closing animation is done playling. This could be done via Animation Notifys or to get the animation instance and exectute this on completion, but this would add unnaccisary overhead, which is not needed for this demonstration.
  (`/Game/Blueprints/Elevator/elevatorRoom/BP_ElevatorRoom.OpenDoors` (`self.BP Elevator Room`))
  (`KismetSystemLibrary.Delay` 3.0)
  (`self.UpdateDoorStatus` true))

(event `self.CloseElevatorRoomDoors`
  ;[1 1 1] This handels the opening/closing of the Elevator Rooms doors. There is A Delay to wait for before the updated status is send to the SCCharts wrapper function UpdateDoorStatus to make sure the closing animation is done playling. This could be done via Animation Notifys or to get the animation instance and exectute this on completion, but this would add unnaccisary overhead, which is not needed for this demonstration.
  (`/Game/Blueprints/Elevator/elevatorRoom/BP_ElevatorRoom.CloseDoors` (`self.BP Elevator Room`))
  (`KismetSystemLibrary.Delay` 3.0)
  (`self.UpdateDoorStatus` false))

(event `self.ReceiveTick`
  (params (DeltaSeconds :type "Float (single-precision)"))
  (bind _image_0 (`/Game/InteractionWidgets/Blueprints/HUD/BP_SCChartsDisplay.Image_0` (`self.SCChartsDisplay`)))
  (bind _image_0_2 (`/Game/InteractionWidgets/Blueprints/HUD/BP_SCChartsDisplay.Image_0` (`self.SCChartsDisplay`)))
  ;[1 1 1] Debug only
  (if (!= (`self.prevState`) (`self.DebugStateID`))
    (bind _output_get (set `self.prevState` (`self.DebugStateID`)))
    (switch `int` _output_get
      (:`1`
        (`Image.SetBrushFromTexture` _image_0_2 "/Game/Blueprints/Elevator/SCChartsImages/Elevator-IdleOpenDoors.Elevator-IdleOpenDoors" false))
      (:`2`
        (`Image.SetBrushFromTexture` _image_0_2 "/Game/Blueprints/Elevator/SCChartsImages/Elevator-IdleWaitForInput-AfterCloseDoors.Elevator-IdleWaitForInput-AfterCloseDoors" false)
        (`KismetSystemLibrary.Delay` 2.0)
        (`Image.SetBrushFromTexture` _image_0 "/Game/Blueprints/Elevator/SCChartsImages/Elevator-IdleWaitForInput.Elevator-IdleWaitForInput" false))
      (:`3`
        (`Image.SetBrushFromTexture` _image_0_2 "/Game/Blueprints/Elevator/SCChartsImages/Elevator-IdleCloseDoors-AfterWait.Elevator-IdleCloseDoors-AfterWait" false)
        (`KismetSystemLibrary.Delay` 2.0)
        (`Image.SetBrushFromTexture` _image_0 "/Game/Blueprints/Elevator/SCChartsImages/Elevator-IdleCloseDoors.Elevator-IdleCloseDoors" false))
      (:`4`
        (`Image.SetBrushFromTexture` _image_0_2 "/Game/Blueprints/Elevator/SCChartsImages/Elevator-MovingUpAfterReady.Elevator-MovingUpAfterReady" false)
        (`KismetSystemLibrary.Delay` 2.0)
        (`Image.SetBrushFromTexture` _image_0 "/Game/Blueprints/Elevator/SCChartsImages/Elevator-MovingUp.Elevator-MovingUp" false))
      (:`5`
        (`Image.SetBrushFromTexture` _image_0_2 "/Game/Blueprints/Elevator/SCChartsImages/Elevator-MovingDownAfterRdy.Elevator-MovingDownAfterRdy" false)
        (`KismetSystemLibrary.Delay` 2.0)
        (`Image.SetBrushFromTexture` _image_0 "/Game/Blueprints/Elevator/SCChartsImages/Elevator-MovingDown.Elevator-MovingDown" false)))))

(event `self.ReceiveBeginPlay`
  ;[1 1 1] Debug only
  (bind _returnvalue (`|CreateWidget` "/Game/InteractionWidgets/Blueprints/HUD/BP_SCChartsDisplay.BP_SCChartsDisplay_C" (`GameplayStatics.GetPlayerController` 0)))
  (`UserWidget.AddToViewport` _returnvalue 0)
  (set `self.SCChartsDisplay` _returnvalue))

(fn `SetStatus`
  (params (Floor :type Integer) (On :type Boolean) (IsInside :type Boolean))
  (bind _returnvalue (!= Floor (`self.CurrentFloor`)))
  (if IsInside
    (if _returnvalue
      (`/Game/Blueprints/Elevator/elevatorRoom/BP_ElevatorRoom.SetStatus` (`self.BP Elevator Room`) Floor On))
    (elif _returnvalue
      (switch `int` Floor
        (:`0`
          (bind _asbp_btn_base (cast `/Game/Blueprints/Elevator/BbtnPanel/BP_BtnBase` (`ChildActorComponent.ChildActor` (`self.BP_BtnUpOutside`))))
          (`/Game/Blueprints/Elevator/BbtnPanel/BP_BtnBase.SetStatus` _asbp_btn_base On))
        (:`1`
          (bind _asbp_btn_base_2 (cast `/Game/Blueprints/Elevator/BbtnPanel/BP_BtnBase` (`ChildActorComponent.ChildActor` (`self.BP_BtnUpOutside1`))))
          (`/Game/Blueprints/Elevator/BbtnPanel/BP_BtnBase.SetStatus` _asbp_btn_base_2 On))
        (:`2`
          (bind _asbp_btn_base_3 (cast `/Game/Blueprints/Elevator/BbtnPanel/BP_BtnBase` (`ChildActorComponent.ChildActor` (`self.BP_BtnUpOutside2`))))
          (`/Game/Blueprints/Elevator/BbtnPanel/BP_BtnBase.SetStatus` _asbp_btn_base_3 On))))))

(fn `UserConstructionScript`
  (bind _bp_btnupoutside (`self.BP_BtnUpOutside`))
  (bind _bp_btnupoutside1 (`self.BP_BtnUpOutside1`))
  (bind _bp_btnupoutside2 (`self.BP_BtnUpOutside2`))
  (`|ExecutionSequence`
    (:`then_0`
      (`/Engine/EditorBlueprintResources/StandardMacros.IsValid` _bp_btnupoutside
        (:`Is Valid`
          (bind _asbp_btn_up_outside (cast `/Game/Blueprints/Elevator/BbtnPanel/BP_BtnUpOutside` (`ChildActorComponent.ChildActor` _bp_btnupoutside)))
          (set `/Game/Blueprints/Elevator/BbtnPanel/BP_BtnBase.Elevator` self _asbp_btn_up_outside)
          (`/Engine/EditorBlueprintResources/StandardMacros.IsValid` _bp_btnupoutside1
            (:`Is Valid`
              (bind _asbp_btn_up_outside_2 (cast `/Game/Blueprints/Elevator/BbtnPanel/BP_BtnUpOutside` (`ChildActorComponent.ChildActor` _bp_btnupoutside1)))
              (set `/Game/Blueprints/Elevator/BbtnPanel/BP_BtnBase.Elevator` self _asbp_btn_up_outside_2)
              (`/Engine/EditorBlueprintResources/StandardMacros.IsValid` _bp_btnupoutside2
                (:`Is Valid`
                  (bind _asbp_btn_up_outside_3 (cast `/Game/Blueprints/Elevator/BbtnPanel/BP_BtnUpOutside` (`ChildActorComponent.ChildActor` _bp_btnupoutside2)))
                  (set `/Game/Blueprints/Elevator/BbtnPanel/BP_BtnBase.Elevator` self _asbp_btn_up_outside_3))))))))
    (:`then_1`
      (bind _asbp_elevator_door_outside (cast `/Game/Blueprints/Elevator/DoorsOuter/BP_ElevatorDoorOutside` (`ChildActorComponent.ChildActor` (`self.BP_ElevatorDoorOutside0`))))
      (set `self.DoorsAtFloor0` _asbp_elevator_door_outside))
    (:`then_2`
      (bind _asbp_elevator_door_outside_2 (cast `/Game/Blueprints/Elevator/DoorsOuter/BP_ElevatorDoorOutside` (`ChildActorComponent.ChildActor` (`self.BP_ElevatorDoorOutside1`))))
      (set `self.DoorsAtFloor1` _asbp_elevator_door_outside_2))
    (:`then_3`
      (bind _asbp_elevator_door_outside_3 (cast `/Game/Blueprints/Elevator/DoorsOuter/BP_ElevatorDoorOutside` (`ChildActorComponent.ChildActor` (`self.BP_ElevatorDoorOutside2`))))
      (set `self.DoorsAtFloor2` _asbp_elevator_door_outside_3))
    (:`then_4`
      (bind _asbp_elevator_room (cast `/Game/Blueprints/Elevator/elevatorRoom/BP_ElevatorRoom` (`ChildActorComponent.ChildActor` (`self.BP_ElevatorRoom`))))
      (bind _output_get (set `self.BP Elevator Room` _asbp_elevator_room))
      (set `/Game/Blueprints/Elevator/elevatorRoom/BP_ElevatorRoom.BP_Elevator` self _output_get)
      (`/Game/Blueprints/Elevator/elevatorRoom/BP_ElevatorRoom.SetReferences` _output_get))
    (:`then_5`
      (`|ExecutionSequence`
        (:`then_0`
          (bind _asbp_btn_base (cast `/Game/Blueprints/Elevator/BbtnPanel/BP_BtnBase` (`ChildActorComponent.ChildActor` (`self.BP_BtnUpOutside`))))
          (set `/Game/Blueprints/Elevator/BbtnPanel/BP_BtnBase.Elevator` self _asbp_btn_base))
        (:`then_1`
          (bind _asbp_btn_base_2 (cast `/Game/Blueprints/Elevator/BbtnPanel/BP_BtnBase` (`ChildActorComponent.ChildActor` (`self.BP_BtnUpOutside1`))))
          (set `/Game/Blueprints/Elevator/BbtnPanel/BP_BtnBase.Elevator` self _asbp_btn_base_2))
        (:`then_2`
          (bind _asbp_btn_base_3 (cast `/Game/Blueprints/Elevator/BbtnPanel/BP_BtnBase` (`ChildActorComponent.ChildActor` (`self.BP_BtnUpOutside2`))))
          (set `/Game/Blueprints/Elevator/BbtnPanel/BP_BtnBase.Elevator` self _asbp_btn_base_3))))))