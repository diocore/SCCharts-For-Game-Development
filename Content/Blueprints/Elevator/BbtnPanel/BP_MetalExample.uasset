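; BP_MetalExample is an example metal resource pickup that supplies the content for its on-screen info widget.
; It overrides the parent's widget functions to set title, subtitle, amount, rarity level and a Pickup key prompt.
; Widget colors come from the Common row of the QualitysColors data table.
; The file holds no pickup logic of its own, and its construction script only calls the parent.
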(fn `Set Widget Amount`
  (returns (`Return Value` :type Boolean) (`Amount Value` :type Integer))
  (return true 100))

(fn `Set Widget Color`
  (returns (`Dark Color` :type "LinearColor Structure") (`Light Color` :type "LinearColor Structure"))
  (bind (_return_value _dark_color _light_color) (`/Game/InteractionWidgets/Blueprints/Libraries/InteractionFunctions.Get Quality Color` (make `DataTableRowHandle` "/Game/InteractionWidgets/Blueprints/QualitysColors.QualitysColors" "Common")))
  (return _dark_color _light_color))

(fn `Set Widget Key Binds`
  (returns (`Return Value` :type Boolean) (`Key Binds` :type "Array of /Game/InteractionWidgets/Blueprints/Stucts/S_KeyBinds Structure"))
  (return true (`|MakeArray` (make `/Game/InteractionWidgets/Blueprints/Stucts/S_KeyBinds` "E" "Pickup") :!type "/Game/InteractionWidgets/Blueprints/Stucts/S_KeyBinds Structure")))

(fn `Set Widget Level`
  (returns (`Return Value` :type Boolean) (`Level Text` :type Text))
  (return true "Common"))

(fn `Set Widget Sub Title`
  (returns (`Return Value` :type Boolean) (`Sub Title Text` :type Text))
  (return true "Resource"))

(fn `Set Widget Title`
  (returns (`Return Value` :type Boolean) (`Title Text` :type Text))
  (return true "Metal"))

(fn `UserConstructionScript`
  (`parent.UserConstructionScript`))