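; Base elevator button actor that, on interact, plays a press animation, briefly hides its label and reports its floor to the linked elevator.
; The elevator receives PressBtn, which a comment says feeds a C++ SCChart wrapper, plus a floor status update.
; Target events forward to a child-actor interaction widget, configured through getters for title and E key prompt.
; SetStatus swaps on/off materials, and construction sets the label text.
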(event `/Game/InteractionWidgets/Blueprints/Interfaces/InteractionInterface.Current Target`
  (params (Pawn :type "Pawn Object Reference"))
  (bind _childactor (`ChildActorComponent.ChildActor` (`self.Widget`)))
  ;[1 1 1] Current target (Copy and paste this in to your own actor)
  (message `/Game/InteractionWidgets/Blueprints/Interfaces/InteractionInterface.Current Target` _childactor Pawn)
  (message `/Game/InteractionWidgets/Blueprints/Interfaces/InteractionInterface.ParentActor` _childactor self))

(event `/Game/InteractionWidgets/Blueprints/Interfaces/InteractionInterface.Clear Target`
  ;[1 1 1] Clear target (Copy and paste this in to your own actor)
  (message `/Game/InteractionWidgets/Blueprints/Interfaces/InteractionInterface.Clear Target` (`ChildActorComponent.ChildActor` (`self.Widget`))))

(event `/Game/InteractionWidgets/Blueprints/Interfaces/InteractionInterface.Interact`
  (params (Key :type "Key Structure") (Pawn :type "Pawn Object Reference"))
  (bind _elevator (`self.Elevator`))
  (bind _floor (`self.Floor`))
  ;[1 1 1] This only plays the button press animation
  (`SkeletalMeshComponent.PlayAnimation` (`self.Button`) "/Game/Blueprints/Elevator/BbtnPanel/newButton/Button_Square_high_Anim_Button_Square_ARMT_Button_Pressed_Up_001.Button_Square_high_Anim_Button_Square_ARMT_Button_Pressed_Up_001" false)
  (`SceneComponent.SetVisibility` (`self.TextRender`) false false)
  (`KismetSystemLibrary.Delay` 0.3)
  (`SceneComponent.SetVisibility` (`self.TextRender`) true false)
  ;[1 1 1] This sends the PressBtnDown signal to the c++ SCChart wrapper after calling the Parent event Interact, which plays the press Animation
  (`/Engine/EditorBlueprintResources/StandardMacros.IsValid` _elevator
    (:`Is Valid`
      (`MyActor.PressBtn` _elevator _floor)
      (`/Game/Blueprints/Elevator/BP_Elevator.SetStatus` (`self.Elevator`) _floor true (`self.IsInside`)))))

(fn `Set Detail 1`
  (returns (`Return Value` :type Boolean) (`Detail Settings` :type "/Game/InteractionWidgets/Blueprints/Stucts/S_DetailsSettings Structure"))
  (return false))

(fn `Set Detail 2`
  (returns (`Return Value` :type Boolean) (`Detail Settings` :type "/Game/InteractionWidgets/Blueprints/Stucts/S_DetailsSettings Structure"))
  (return false))

(fn `Set Detail 3`
  (returns (`Return Value` :type Boolean) (`Detail Settings` :type "/Game/InteractionWidgets/Blueprints/Stucts/S_DetailsSettings Structure"))
  (return false))

(fn `Set Detail 4`
  (returns (`Return Value` :type Boolean) (`Detail Settings` :type "/Game/InteractionWidgets/Blueprints/Stucts/S_DetailsSettings Structure"))
  (return false))

(fn `Set Widget Amount`
  (returns (`Return Value` :type Boolean) (`Amount Value` :type Integer))
  (return false 0))

(fn `Set Widget Color`
  (returns (`Dark Color` :type "LinearColor Structure") (`Light Color` :type "LinearColor Structure"))
  (bind (_return_value _dark_color _light_color) (`/Game/InteractionWidgets/Blueprints/Libraries/InteractionFunctions.Get Quality Color` (make `DataTableRowHandle` "/Game/InteractionWidgets/Blueprints/QualitysColors.QualitysColors" "Common")))
  (return _dark_color _light_color))

(fn `Set Widget Key Binds`
  (returns (`Return Value` :type Boolean) (`Key Binds` :type "Array of /Game/InteractionWidgets/Blueprints/Stucts/S_KeyBinds Structure"))
  (return true (`|MakeArray` (make `/Game/InteractionWidgets/Blueprints/Stucts/S_KeyBinds` "E" (`KismetSystemLibrary.MakeLiteralText` (`self.Btn_text`))) :!type "/Game/InteractionWidgets/Blueprints/Stucts/S_KeyBinds Structure")))

(fn `Set Widget Level`
  (returns (`Return Value` :type Boolean) (`Level Text` :type Text))
  (return false ""))

(fn `Set Widget Sub Title`
  (returns (`Return Value` :type Boolean) (`Sub Title Text` :type Text))
  (return false ""))

(fn `Set Widget Title`
  (returns (`Return Value` :type Boolean) (`Title Text` :type Text))
  (return true (`self.Btn_text`)))

(fn `Set Widget Type`
  (returns (`Widget Type` :type "/Game/InteractionWidgets/Blueprints/Enums/E_WidgetTypes Enum"))
  (return "NewEnumerator2"))

(fn `SetStatus`
  (params (On :type Boolean))
  (bind _button (`self.Button`))
  (if On
    (`PrimitiveComponent.SetMaterial` _button 0 "/Game/Blueprints/Elevator/BbtnPanel/newButton/Material_On.Material_On")
    (else
      (`PrimitiveComponent.SetMaterial` _button 0 "/Game/Blueprints/Elevator/BbtnPanel/newButton/Material_Off.Material_Off"))))

(fn `UserConstructionScript`
  (`TextRenderComponent.K2_SetText` (`self.TextRender`) (`self.Label`)))