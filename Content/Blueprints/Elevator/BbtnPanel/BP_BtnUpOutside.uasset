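; Outside "Up" call button for an elevator, an interactable actor with an on-screen prompt widget.
; Interact runs the parent event for the press animation, then passes its Floor to the C++ CallElevator on a valid Elevator, which queues it.
; Target and clear events forward to the Widget child actor, while override functions give it the title, E key bind and Common quality colors, leaving other fields off.
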(event `/Game/InteractionWidgets/Blueprints/Interfaces/InteractionInterface.Current Target`
  (params (Pawn :type "Pawn Object Reference"))
  (bind _childactor (`ChildActorComponent.ChildActor` (`self.Widget`)))
  ;[1 1 1] Current target (Copy and paste this in to your own actor)
  (message `/Game/InteractionWidgets/Blueprints/Interfaces/InteractionInterface.Current Target` _childactor Pawn)
  (message `/Game/InteractionWidgets/Blueprints/Interfaces/InteractionInterface.ParentActor` _childactor self))

(event `/Game/InteractionWidgets/Blueprints/Interfaces/InteractionInterface.Clear Target`
  ;[1 1 1] Clear target (Copy and paste this in to your own actor)
  (message `/Game/InteractionWidgets/Blueprints/Interfaces/InteractionInterface.Clear Target` (`ChildActorComponent.ChildActor` (`self.Widget`))))

(event `/Game/InteractionWidgets/Blueprints/Interfaces/InteractionInterface.Interact`
  (params (Key :type "Key Structure") (Pawn :type "Pawn Object Reference"))
  (bind _elevator (`self.Elevator`))
  ;[1 1 1] This calls the CallElevator() function in c++ end enqueues the Floor that it was pressed on to the Elevator Queue after calling the Parent event Interact, which plays the press Animation
  (`parent.Interact` (struct) null)
  (`/Engine/EditorBlueprintResources/StandardMacros.IsValid` _elevator
    (:`Is Valid`
      (`MyActor.CallElevator` _elevator (`self.Floor`)))))

(fn `Set Detail 1`
  (returns (`Return Value` :type Boolean) (`Detail Settings` :type "/Game/InteractionWidgets/Blueprints/Stucts/S_DetailsSettings Structure"))
  (return false))

(fn `Set Detail 2`
  (returns (`Return Value` :type Boolean) (`Detail Settings` :type "/Game/InteractionWidgets/Blueprints/Stucts/S_DetailsSettings Structure"))
  (return false))

(fn `Set Detail 3`
  (returns (`Return Value` :type Boolean) (`Detail Settings` :type "/Game/InteractionWidgets/Blueprints/Stucts/S_DetailsSettings Structure"))
  (return false))

(fn `Set Detail 4`
  (returns (`Return Value` :type Boolean) (`Detail Settings` :type "/Game/InteractionWidgets/Blueprints/Stucts/S_DetailsSettings Structure"))
  (return false))

(fn `Set Widget Amount`
  (returns (`Return Value` :type Boolean) (`Amount Value` :type Integer))
  (return false 0))

(fn `Set Widget Color`
  (returns (`Dark Color` :type "LinearColor Structure") (`Light Color` :type "LinearColor Structure"))
  (bind (_return_value _dark_color _light_color) (`/Game/InteractionWidgets/Blueprints/Libraries/InteractionFunctions.Get Quality Color` (make `DataTableRowHandle` "/Game/InteractionWidgets/Blueprints/QualitysColors.QualitysColors" "Common")))
  (return _dark_color _light_color))

(fn `Set Widget Key Binds`
  (returns (`Return Value` :type Boolean) (`Key Binds` :type "Array of /Game/InteractionWidgets/Blueprints/Stucts/S_KeyBinds Structure"))
  (return true (`|MakeArray` (make `/Game/InteractionWidgets/Blueprints/Stucts/S_KeyBinds` "E" "") :!type "/Game/InteractionWidgets/Blueprints/Stucts/S_KeyBinds Structure")))

(fn `Set Widget Level`
  (returns (`Return Value` :type Boolean) (`Level Text` :type Text))
  (return false ""))

(fn `Set Widget Sub Title`
  (returns (`Return Value` :type Boolean) (`Sub Title Text` :type Text))
  (return false ""))

(fn `Set Widget Title`
  (returns (`Return Value` :type Boolean) (`Title Text` :type Text))
  (return true "Up"))

(fn `Set Widget Type`
  (returns (`Widget Type` :type "/Game/InteractionWidgets/Blueprints/Enums/E_WidgetTypes Enum"))
  (return "NewEnumerator2"))

(fn `UserConstructionScript`)