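; BP_BtnUp is the elevator panel's up button, supplying the content for its on-screen widget.
; Widget setter functions return BtnText as both the title and the E key bind label, with colors from the Common row of the QualitysColors table.
; Subtitle, level, amount and all detail fields are switched off.
; The event graph and construction script are empty, so this Blueprint defines no press behavior itself.
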(fn `Set Detail 1`
  (returns (`Return Value` :type Boolean) (`Detail Settings` :type "/Game/InteractionWidgets/Blueprints/Stucts/S_DetailsSettings Structure"))
  (return false))

(fn `Set Detail 2`
  (returns (`Return Value` :type Boolean) (`Detail Settings` :type "/Game/InteractionWidgets/Blueprints/Stucts/S_DetailsSettings Structure"))
  (return false))

(fn `Set Detail 3`
  (returns (`Return Value` :type Boolean) (`Detail Settings` :type "/Game/InteractionWidgets/Blueprints/Stucts/S_DetailsSettings Structure"))
  (return false))

(fn `Set Detail 4`
  (returns (`Return Value` :type Boolean) (`Detail Settings` :type "/Game/InteractionWidgets/Blueprints/Stucts/S_DetailsSettings Structure"))
  (return false))

(fn `Set Widget Amount`
  (returns (`Return Value` :type Boolean) (`Amount Value` :type Integer))
  (return false 0))

(fn `Set Widget Color`
  (returns (`Dark Color` :type "LinearColor Structure") (`Light Color` :type "LinearColor Structure"))
  (bind (_return_value _dark_color _light_color) (`/Game/InteractionWidgets/Blueprints/Libraries/InteractionFunctions.Get Quality Color` (make `DataTableRowHandle` "/Game/InteractionWidgets/Blueprints/QualitysColors.QualitysColors" "Common")))
  (return _dark_color _light_color))

(fn `Set Widget Key Binds`
  (returns (`Return Value` :type Boolean) (`Key Binds` :type "Array of /Game/InteractionWidgets/Blueprints/Stucts/S_KeyBinds Structure"))
  (return true (`|MakeArray` (make `/Game/InteractionWidgets/Blueprints/Stucts/S_KeyBinds` "E" (`self.Btn_text`)) :!type "/Game/InteractionWidgets/Blueprints/Stucts/S_KeyBinds Structure")))

(fn `Set Widget Level`
  (returns (`Return Value` :type Boolean) (`Level Text` :type Text))
  (return false ""))

(fn `Set Widget Sub Title`
  (returns (`Return Value` :type Boolean) (`Sub Title Text` :type Text))
  (return false ""))

(fn `Set Widget Title`
  (returns (`Return Value` :type Boolean) (`Title Text` :type Text))
  (return true (`self.Btn_text`)))

(fn `Set Widget Type`
  (returns (`Widget Type` :type "/Game/InteractionWidgets/Blueprints/Enums/E_WidgetTypes Enum"))
  (return "NewEnumerator2"))

(fn `UserConstructionScript`)