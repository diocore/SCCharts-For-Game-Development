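; BP_ElevatorRoom is the moving elevator cabin, with child-actor inner doors, up to three floor buttons and a screen.
; Its construction script caches buttons and screen, and BeginPlay gives the buttons the parent elevator reference.
; MoveElevator offsets Z by 1000 units per floor for a Timeline lerp, while the screen shows direction.
; On finish, it updates the floor, reports it to BPElevator for the SCCharts state machine and displays it.
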(event `self.ReceiveBeginPlay`
  (`self.SetElevatorRef` (`self.BP_Elevator`)))

(event `self.ReceiveTick`
  (params (DeltaSeconds :type "Float (single-precision)")))

(event `HandleMovement`
  (params (Up :type Boolean) (Floors :type Integer) (TargetLocation :type "Vector Structure"))
  (bind _currentfloor (`self.CurrentFloor`))
  (bind _screen (`self.Screen`))
  (bind _bp_elevator (`self.BP_Elevator`))
  ;[1 1 1] This moves the Elevator Room with a Timeline node and after the movement has finished it updates the current floor for the SCCharts state Machiene
  (bind (_direction _newtrack_2) (`Timeline|Timeline` :!via `PlayFromStart`)
    (:`Update`
      (if Up
        (`/Game/Blueprints/Elevator/elevatorRoom/BP_Screen.Set Text` _screen "UP" 10.0)
        (else
          (`/Game/Blueprints/Elevator/elevatorRoom/BP_Screen.Set Text` _screen "DOWN" 10.0)))
      (`self.K2_SetActorLocation` (`KismetMathLibrary.VLerp` (`self.K2_GetActorLocation`) TargetLocation _newtrack_2)))
    (:`Finished`
      (if Up
        (bind _output_get (set `self.CurrentFloor` (+ _currentfloor Floors)))
        (`MyActor.UpdateFloorStatus` _bp_elevator _output_get)
        (else
          (bind _output_get_2 (set `self.CurrentFloor` (- _currentfloor Floors)))
          (`MyActor.UpdateFloorStatus` _bp_elevator _output_get_2)))
      (`/Game/Blueprints/Elevator/elevatorRoom/BP_Screen.Set Text` (`self.Screen`) (`KismetTextLibrary.Conv_IntToText` (`self.CurrentFloor`)) 26.0))))

(event `MoveElevator`
  (params (Up :type Boolean) (NumFloors :type Integer))
  (bind (_returnvalue_x _returnvalue_y _returnvalue_z) (`KismetMathLibrary.BreakVector` (`self.K2_GetActorLocation`)))
  (bind (_returnvalue_x_2 _returnvalue_y_2 _returnvalue_z_2) (`KismetMathLibrary.BreakVector` (`self.K2_GetActorLocation`)))
  ;[1 1 1] This starts the Elevator Room movement. It determins wether the elevator should move up or down from the input "up" and how many floors it should move and to what Location and sends the information to the HandleMovement Event.
  (if Up
    (`self.HandleMovement` true NumFloors (`KismetMathLibrary.MakeVector` _returnvalue_x _returnvalue_y (+ _returnvalue_z (`KismetMathLibrary.Conv_IntToDouble` (* NumFloors 1000)))))
    (else
      (`self.HandleMovement` false NumFloors (`KismetMathLibrary.MakeVector` _returnvalue_x_2 _returnvalue_y_2 (+ _returnvalue_z_2 (`KismetMathLibrary.Conv_IntToDouble` (* NumFloors -1000))))))))

(fn `CloseDoors`
  (bind _childactor (`ChildActorComponent.ChildActor` (`self.BP_ElevatorDoorsInner`)))
  (`/Engine/EditorBlueprintResources/StandardMacros.IsValid` _childactor
    (:`Is Valid`
      (bind _asbp_elevator_doors_inner (cast `/Game/Blueprints/Elevator/DoorsInner/BP_ElevatorDoorsInner` _childactor))
      (`/Game/Blueprints/Elevator/DoorsInner/BP_ElevatorDoorsInner.CloseDoors` _asbp_elevator_doors_inner))))

(fn `OpenDoors`
  (bind _childactor (`ChildActorComponent.ChildActor` (`self.BP_ElevatorDoorsInner`)))
  (`/Engine/EditorBlueprintResources/StandardMacros.IsValid` _childactor
    (:`Is Valid`
      (bind _asbp_elevator_doors_inner (cast `/Game/Blueprints/Elevator/DoorsInner/BP_ElevatorDoorsInner` _childactor))
      (`/Game/Blueprints/Elevator/DoorsInner/BP_ElevatorDoorsInner.OpenDoors` _asbp_elevator_doors_inner))))

(fn `SetElevatorRef`
  (params (NewParam :type "/Game/Blueprints/Elevator/BP_Elevator Object Reference"))
  (`|ExecutionSequence`
    (:`then_0`
      (set `/Game/Blueprints/Elevator/BbtnPanel/BP_BtnBase.Elevator` NewParam (`self.Btn_1`)))
    (:`then_1`
      (set `/Game/Blueprints/Elevator/BbtnPanel/BP_BtnBase.Elevator` NewParam (`self.Btn_2`)))
    (:`then_2`
      (set `/Game/Blueprints/Elevator/BbtnPanel/BP_BtnBase.Elevator` NewParam (`self.Btn_3`)))))

(fn `SetReferences`
  (bind _bp_elevator (`self.BP_Elevator`))
  (`|ExecutionSequence`
    (:`then_0`
      (set `/Game/Blueprints/Elevator/BbtnPanel/BP_BtnUp.Elevator` _bp_elevator (`self.Btn_1`)))
    (:`then_1`
      (set `/Game/Blueprints/Elevator/BbtnPanel/BP_BtnDown.Elevator` _bp_elevator (`self.Btn_2`)))))

(fn `SetStatus`
  (params (Floor :type Integer) (On :type Boolean))
  (switch `int` Floor
    (:`0`
      (`/Game/Blueprints/Elevator/BbtnPanel/BP_BtnBase.SetStatus` (`self.Btn_1`) On))
    (:`1`
      (`/Game/Blueprints/Elevator/BbtnPanel/BP_BtnBase.SetStatus` (`self.Btn_2`) On))
    (:`2`
      (`/Game/Blueprints/Elevator/BbtnPanel/BP_BtnBase.SetStatus` (`self.Btn_3`) On))))

(fn `UserConstructionScript`
  (bind _bp_btn2 (`self.BP_Btn2`))
  (bind _bp_btn3 (`self.BP_Btn3`))
  (`|ExecutionSequence`
    (:`then_0`
      (bind _asbp_btn_base (cast `/Game/Blueprints/Elevator/BbtnPanel/BP_BtnBase` (`ChildActorComponent.ChildActor` (`self.BP_Btn1`))))
      (set `self.Btn_1` _asbp_btn_base))
    (:`then_1`
      (`/Engine/EditorBlueprintResources/StandardMacros.IsValid` _bp_btn2
        (:`Is Valid`
          (bind _asbp_btn_base_2 (cast `/Game/Blueprints/Elevator/BbtnPanel/BP_BtnBase` (`ChildActorComponent.ChildActor` _bp_btn2)))
          (set `self.Btn_2` _asbp_btn_base_2))))
    (:`then_2`
      (`/Engine/EditorBlueprintResources/StandardMacros.IsValid` _bp_btn3
        (:`Is Valid`
          (bind _asbp_btn_base_3 (cast `/Game/Blueprints/Elevator/BbtnPanel/BP_BtnBase` (`ChildActorComponent.ChildActor` _bp_btn3)))
          (set `self.Btn_3` _asbp_btn_base_3))))
    (:`then_3`
      (bind _asbp_screen (cast `/Game/Blueprints/Elevator/elevatorRoom/BP_Screen` (`ChildActorComponent.ChildActor` (`self.BP_Screen`))))
      (set `self.Screen` _asbp_screen))))