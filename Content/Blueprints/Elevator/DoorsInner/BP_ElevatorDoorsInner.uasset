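; BP_ElevatorDoorsInner is the Blueprint for an elevator's inner doors, exposing OpenDoors and CloseDoors functions.
; Each function updates the Open flag, then passes the state to the AB_ElevatorDoorInner anim instance on the ElevatorDoors component.
; The event graph and construction script are empty, so the doors change state only when those functions are called.
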(fn `CloseDoors`
  (bind _output_get (set `self.bOpen` false))
  (bind _asab_elevator_door_inner (cast `/Game/Blueprints/Elevator/DoorsInner/AB_ElevatorDoorInner` (`SkeletalMeshComponent.GetAnimInstance` (`self.ElevatorDoors`))))
  (set `/Game/Blueprints/Elevator/DoorsInner/AB_ElevatorDoorInner.bOpen` _output_get _asab_elevator_door_inner))

(fn `OpenDoors`
  (set `self.bOpen` true)
  (bind _asab_elevator_door_inner (cast `/Game/Blueprints/Elevator/DoorsInner/AB_ElevatorDoorInner` (`SkeletalMeshComponent.GetAnimInstance` (`self.ElevatorDoors`))))
  (set `/Game/Blueprints/Elevator/DoorsInner/AB_ElevatorDoorInner.bOpen` true _asab_elevator_door_inner))

(fn `UserConstructionScript`)